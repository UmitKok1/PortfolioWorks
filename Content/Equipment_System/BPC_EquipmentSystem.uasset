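; BPC_EquipmentSystem is a component on the third-person character that handles weapon pickup, dropping and the equipment menu.
; Interact sphere-traces from the camera, records the weapon's item data in WeaponSlots and attaches it to a data-table-defined mesh socket.
; Drop detaches the held weapon beside the player and removes a slot by array length, not item.
; The menu input toggles WBP_Equipment, input mode and character movement.
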(event EventBeginPlay
  (bind _asbp_third_person_character (Utilities|Casting|CastToBP_ThirdPersonCharacter (Components|GetOwner)))
  (Variables|Default|SetFollow%20Camera (Variables|/Game/ThirdPerson/Blueprints/BP_ThirdPersonCharacter.BP_ThirdPersonCharacter_C|GetFollowCamera _asbp_third_person_character))
  (Variables|Default|SetMesh (Variables|/Script/Engine.Character|GetMesh _asbp_third_person_character)))

(event EventTick
  (params (DeltaSeconds :type Float%20%28single-precision%29)))

(event Input|ActionEvents|InputActionIA_Interact
  (params (Key :type Key%20Structure :default "None"))
  (bind _follow_camera (Variables|Default|GetFollow%20Camera))
  (bind _returnvalue (Transformation|GetWorldLocation _follow_camera))
  (:Pressed
    (bind (_outhit _returnvalue_2) (Collision|SphereTraceForObjects _returnvalue (+ _returnvalue (* (Math|Vector|GetForwardVector (Transformation|GetWorldRotation _follow_camera)) 1e+03)) 3e+01 (Utilities|Array|MakeArray "ObjectTypeQuery2") false 0 "ForDuration"))
    (if _returnvalue_2
      (bind _asbp_weapon (Utilities|Casting|CastToBP_Weapon (.HitActor (Collision|BreakHitResult _outhit))))
      (Variables|Default|Setheld%20item _asbp_weapon)
      (CallFunction|AddWeapon (Variables|/Game/Equipment_System/BP_Weapon.BP_Weapon_C|GetItemData (Variables|Default|Getheld%20item)))
      (bind _returnvalue_3 (Utilities|GetDataTableRow (.datatable (.item (Variables|/Game/Equipment_System/BP_Weapon.BP_Weapon_C|GetItemData (Variables|Default|Getheld%20item)))) (.rowname (.item (Variables|/Game/Equipment_System/BP_Weapon.BP_Weapon_C|GetItemData (Variables|Default|Getheld%20item)))))
        (:then
          (Transformation|AttachComponentToComponent (Variables|Default|Getheld%20item) (Variables|Default|GetMesh) (.SocketName (Utilities|Struct|BreakS_Weapons _returnvalue_3)) "SnapToTarget" "SnapToTarget" "SnapToTarget" true)
          (Collision|SetCollisionEnabled (Variables|/Game/Equipment_System/BP_Weapon.BP_Weapon_C|GetStaticMesh (Variables|Default|Getheld%20item)) "NoCollision")
          (Variables|Default|SetisHolding true))))))

(event Input|ActionEvents|InputActionIA_Drop
  (params (Key :type Key%20Structure :default "None"))
  (bind _returnvalue (Game|Player|GetPlayerPawn 0))
  (:Pressed
    (if (Variables|Default|GetisHolding)
      (Transformation|DetachFromActor (Variables|Default|Getheld%20item) "KeepWorld" "KeepWorld" "KeepWorld")
      (Transformation|SetActorLocationAndRotation (Variables|Default|Getheld%20item) (+ (Transformation|GetActorLocation _returnvalue) (* (Transformation|GetActorRightVector _returnvalue) 1e+02) ""))
      (Variables|Default|SetisHolding false)
      (Collision|SetCollisionProfileName (Variables|/Game/Equipment_System/BP_Weapon.BP_Weapon_C|GetStaticMesh (Variables|Default|Getheld%20item)) "DroppedWeapon" true :!class /Script/Engine.PrimitiveComponent)
      (CallFunction|DropWeapon (Variables|Default|Getheld%20item)))))

(event Input|ActionEvents|InputActionEquipmentMenu
  (params (Key :type Key%20Structure :default "None"))
  (bind _returnvalue (Game|GetPlayerController 0))
  ;[1 1 1] Equipment Menu Panel
  (:Pressed
    (if (not (Variables|Default|GetisPanelOpened))
      (Variables|Default|SetisPanelOpened true)
      (bind _returnvalue_2 (UserInterface|CreateWidget "/Game/Equipment_System/UI/WBP_Equipment.WBP_Equipment_C"))
      (bind _output_get (Variables|Default|SetEquipment%20Widget _returnvalue_2))
      (UserInterface|Viewport|AddtoViewport _output_get 0)
      (Variables|/Script/Engine.PlayerController|SetbShowMouseCursor _returnvalue false)
      (Input|SetInputModeGameandUI _returnvalue (Variables|Default|GetEquipment%20Widget) "DoNotLock" true)
      (bind _asbp_third_person_character (Utilities|Casting|CastToBP_ThirdPersonCharacter (Components|GetOwner)))
      (Pawn|Components|CharacterMovement|SetMovementMode (Variables|/Script/Engine.Character|GetCharacterMovement _asbp_third_person_character) "MOVE_None" 0)
      (else
        (Variables|Default|SetisPanelOpened false)
        (bind _equipment_widget (Variables|Default|GetEquipment%20Widget)
          (:then
            (Widget|RemovefromParent _equipment_widget)
            (Variables|Default|SetEquipment%20Widget 0)
            (Variables|/Script/Engine.PlayerController|SetbShowMouseCursor _returnvalue true)
            (Input|SetInputModeGameOnly _returnvalue)
            (bind _asbp_third_person_character_2 (Utilities|Casting|CastToBP_ThirdPersonCharacter (Components|GetOwner)))
            (Pawn|Components|CharacterMovement|SetMovementMode (Variables|/Script/Engine.Character|GetCharacterMovement _asbp_third_person_character_2) "MOVE_Walking" 0))
          (:else))))))

(event Input|KeyboardEvents|H
  (params (Key :type Key%20Structure :default "None"))
  (:Pressed
    (for _array_element (Variables|Default|GetweaponSlots)
      (Development|PrintString (Utilities|String|ToString(Name) (.rowname (.item _array_element)))))))

(fn AddWeapon
  (params (NewItem :type S%20Slots%20Structure%20%28by%20ref%29))
  (Utilities|Array|Add (Variables|Default|GetweaponSlots) NewItem))

(fn DropWeapon
  (params (NewParam :type BP%20Weapon%20Object%20Reference))
  (bind _weaponslots (Variables|Default|GetweaponSlots))
  (bind _result (Math|Integer|DecrementInt (Utilities|Array|Length _weaponslots))
    (:%20%20
      (Utilities|Array|RemoveIndex _weaponslots _result))))