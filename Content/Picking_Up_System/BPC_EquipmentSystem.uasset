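; Equipment component for the third-person character that picks up weapons the player looks at and attaches them to the body.
; On interact, a camera-forward sphere trace finds a BP_Weapon and adds its item data to the WeaponSlots array.
; The item's data table row supplies the mesh socket to snap to, and the weapon's collision is disabled.
; The H key prints stored item row names for debugging.
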(event EventBeginPlay
  (bind _asbp_third_person_character (Utilities|Casting|CastToBP_ThirdPersonCharacter (Components|GetOwner)))
  (Variables|Default|SetFollow%20Camera (Variables|/Game/ThirdPerson/Blueprints/BP_ThirdPersonCharacter.BP_ThirdPersonCharacter_C|GetFollowCamera _asbp_third_person_character))
  (Variables|Default|SetMesh (Variables|/Script/Engine.Character|GetMesh _asbp_third_person_character)))

(event EventTick
  (params (DeltaSeconds :type Float%20%28single-precision%29)))

(event Input|ActionEvents|InputActionIA_Interact
  (params (Key :type Key%20Structure :default "None"))
  (bind _follow_camera (Variables|Default|GetFollow%20Camera))
  (bind _returnvalue (Transformation|GetWorldLocation _follow_camera))
  (:Pressed
    (bind (_outhit _returnvalue_2) (Collision|SphereTraceForObjects _returnvalue (+ _returnvalue (* (Math|Vector|GetForwardVector (Transformation|GetWorldRotation _follow_camera)) 1e+03)) 15.0 (Utilities|Array|MakeArray "ObjectTypeQuery2") false 0 "ForDuration"))
    (if _returnvalue_2
      (bind _asbp_weapon (Utilities|Casting|CastToBP_Weapon (.HitActor (Collision|BreakHitResult _outhit))))
      (CallFunction|AddWeapon (Variables|/Game/Picking_Up_System/BP_Weapon.BP_Weapon_C|GetItemData _asbp_weapon))
      (bind _returnvalue_3 (Utilities|GetDataTableRow (.datatable (.item (Variables|/Game/Picking_Up_System/BP_Weapon.BP_Weapon_C|GetItemData _asbp_weapon))) (.rowname (.item (Variables|/Game/Picking_Up_System/BP_Weapon.BP_Weapon_C|GetItemData _asbp_weapon))))
        (:then
          (Collision|SetCollisionEnabled (Variables|/Game/Picking_Up_System/BP_Weapon.BP_Weapon_C|GetStaticMesh _asbp_weapon) "NoCollision")
          (Transformation|AttachComponentToComponent _asbp_weapon (Variables|Default|GetMesh) (.SocketName (Utilities|Struct|BreakS_Weapons _returnvalue_3)) "SnapToTarget" "SnapToTarget" "SnapToTarget" true))))))

(event Input|KeyboardEvents|H
  (params (Key :type Key%20Structure :default "None"))
  (:Pressed
    (for _array_element (Variables|Default|GetweaponSlots)
      (Development|PrintString (Utilities|String|ToString(Name) (.rowname (.item _array_element)))))))

(fn AddWeapon
  (params (NewItem :type S%20Slots%20Structure%20%28by%20ref%29))
  (Utilities|Array|Add (Variables|Default|GetweaponSlots) NewItem))